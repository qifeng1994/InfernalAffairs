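; Camera_BP is a player camera with look controls for a scene of talking to an NPC through fog.
; BeginPlay shows a fog widget, which fades out and is removed when the referenced NPC leaves.
; Space triggers that NPC's DialogComponent, while F calls a left-hand wake-up event for a limited count, then GetMad with a Blank-to-Mad audio crossfade.
; Right-hand wake-up and camera yaw limit logic are left unwired.
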(event Custom|RemoveFogWidget
  (bind _fogwidget (Variables|Default|GetFogWidget))
  ;[1 1 1] when dialog finshed, NPC leave, and remove fog widget
  (Components|Animation|PlayAnimation _fogwidget (Variables|/Game/InfernalAffairs/DialogSystem/FogWidget.FogWidget_C|GetFade _fogwidget) 0.0
    (:Finished
      (Widget|RemovefromParent _fogwidget))))

(event EventBeginPlay
  ;[1 1 1] control for camera rotate
  ;[1 1 1] add a foggy widget
  (bind _returnvalue (UserInterface|CreateWidget "/Game/InfernalAffairs/DialogSystem/FogWidget.FogWidget_C" (Game|GetPlayerController 0)))
  (bind _output_get (Variables|Default|SetFogWidget _returnvalue))
  (UserInterface|Viewport|AddtoViewport _output_get 0)
  ;[1 1 1] when dialog finshed, NPC leave, and remove fog widget
  (EventDispatchers|BindEventtoNPCleaved (Variables|Default|GetNPCreference) (delegate Custom|RemoveFogWidget)))

(event Input|AxisEvents|InputAxisLookUp
  (params (AxisValue :type Float%20%28single-precision%29))
  ;[1 1 1] control for camera rotate
  (Pawn|Input|AddControllerPitchInput AxisValue))

(event Input|AxisEvents|InputAxisTurn
  (params (AxisValue :type Float%20%28single-precision%29))
  ;[1 1 1] control for camera rotate
  (Pawn|Input|AddControllerYawInput AxisValue))

(event Input|MouseEvents|LeftMouseButton
  (params (Key :type Key%20Structure :default "None")))

(event Input|MouseEvents|RightMouseButton
  (params (Key :type Key%20Structure :default "None"))
  ;[1 1 1] press mouse button to call wakeup event and play animation
)

(event Input|KeyboardEvents|SpaceBar
  (params (Key :type Key%20Structure :default "None"))
  ;[1 1 1] press space to talk to NPC1
  (:Pressed
    (Class|DialogInterface|OnInteraction(Message) (Actor|GetComponentbyClass (Variables|Default|GetNPCreference) "/Game/InfernalAffairs/DialogSystem/DialogComponent.DialogComponent_C"))))

(event Input|KeyboardEvents|F
  (params (Key :type Key%20Structure :default "None"))
  ;[1 1 1] press mouse button to call wakeup event and play animation
  (:Pressed
    (if (Variables|Default|GetMontagePlayable)
      (Variables|Default|SetMontageCounter (+ (Variables|Default|GetMontageCounter) 1))
      (if (<= (Variables|Default|GetMontageCounter) 5)
        (Default|CallWakeUpLeftHand)
        (else
          (Variables|Default|SetMontagePlayable false)
          (Default|CallGetMad)
          (Audio|Components|Audio|FadeOut (Variables|Default|GetBlank) 5.0 0.3 "Linear" :!class /Script/Engine.AudioComponent)
          (Audio|Components|Audio|FadeIn (Variables|Default|GetMad) 1.0 0.8 0.0 "Linear" :!class /Script/Engine.AudioComponent))))))

(fn ConstructionScript)